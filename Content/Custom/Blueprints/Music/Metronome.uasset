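; Metronome actor that keeps a four-beat musical count and broadcasts beat starts to listening actors.
; BeginPlay starts a pause-respecting BeatTimeline, whose play rate is set to 60 / BeatsPerMinute and recomputed on every update.
; Each timeline finish advances and prints the zero-based beat, restarts the timeline, then sends the one-based beat via BeatStartMessage to all MusicControllerListener actors.
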(event EventBeginPlay
  (bind _beattimeline (Variables|Default|GetbeatTimeline))
  (CallFunction|AdjustBeatPlayRatebyCurrentBPM)
  (Class|ActorComponent|SetTickablewhenPaused _beattimeline false)
  (Audio|Components|Audio|Play _beattimeline))

(event Collision|EventActorBeginOverlap
  (params (OtherActor :type Actor%20Object%20Reference)))

(fn ConstructionScript)

(fn AdjustBeatPlayRatebyCurrentBPM
  (Components|Timeline|SetPlayRate (Variables|Default|GetbeatTimeline) (/ 1.0 (* (Math|Conversions|ToFloat(Integer) (Variables|Default|GetbeatsPerMinute)) (/ 1.0 6e+01)))))

(fn GetCurrentBeat
  (return (Variables|Default|GetcurrentBeatMinusOne)))