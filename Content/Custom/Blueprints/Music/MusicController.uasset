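; Music controller Blueprint that runs a looping four-beat counter and signals new beats and phrases.
; A restarting Timeline acts as the metronome, with its play rate reset every update to 60 divided by BeatsPerMinute.
; Each finish advances and prints the zero-based beat, signals a phrase on wrap, then restarts and signals the one-based beat.
; Tick separately accumulates time since start.
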(event EventBeginPlay
  (CallFunction|AdjustBeatPlayRatebyCurrentBPM)
  (Timeline|beatTimeline Play
    (:Update
      (CallFunction|AdjustBeatPlayRatebyCurrentBPM))
    (:Finished
      (bind _output_get (Variables|Default|SetcurrentBeatMinusOne (Math|Integer|%(Integer) (+ (Variables|Default|GetcurrentBeatMinusOne) 1) 4)))
      (Utilities|FlowControl|Sequence
        (:then_0
          (bind _currentbeat (CallFunction|GetCurrentBeat))
          (Development|PrintString (Utilities|String|ToString(Integer) _currentbeat)))
        (:then_1
          (if (== _output_get 0)
            (Default|CallSignalNewPhrase)))
        (:then_3
          (Components|Timeline|PlayfromStart (Variables|Default|GetbeatTimeline))
          (Default|CallSignalNewBeat (+ (Variables|Default|GetcurrentBeatMinusOne) 1)))))))

(event Collision|EventActorBeginOverlap
  (params (OtherActor :type Actor%20Object%20Reference)))

(event EventTick
  (params (DeltaSeconds :type Float%20%28single-precision%29))
  (Variables|Default|SettimeSinceStart (+ DeltaSeconds (Variables|Default|GettimeSinceStart))))

(fn ConstructionScript)

(fn AdjustBeatPlayRatebyCurrentBPM
  (Components|Timeline|SetPlayRate (Variables|Default|GetbeatTimeline) (/ 1.0 (* (Math|Conversions|ToFloat(Integer) (Variables|Default|GetbeatsPerMinute)) (/ 1.0 6e+01)))))

(fn GetCurrentBeat
  (return (Variables|Default|GetcurrentBeatMinusOne)))