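; MusicPlayer Blueprint that starts and stops music loop sound cues in step with a beat event.
; Add and remove requests queue cues, and each BeatStart processes stops before spawning 2D sounds for queued cues not already playing.
; A map tracks each cue's audio component, and a MutexLocked flag rejects additions during beat processing.
; Despite the FadeOutAndStopLoopCue name, removal stops and destroys the component without fading.
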(event EventBeatStart
  (params (beat :type Integer))
  (Variables|Default|SetmutexLocked true)
  (CallFunction|StopAllSoundstobeQueued)
  (CallFunction|PlayAllQueuedSounds)
  (Variables|Default|SetmutexLocked false))

(event EventAddSoundCue
  (params (cueToAdd :type Sound%20Cue%20Object%20Reference))
  (CallFunction|QueueSoundtoLoopforNextBeat cueToAdd))

(event EventRemoveSoundCue
  (params (cueToRemove :type Sound%20Cue%20Object%20Reference))
  (CallFunction|FadeOutandStopLoopCue cueToRemove))

(fn ConstructionScript)

(fn QueueSoundtoLoopforNextBeat
  (params (soundCueToQueue :type Sound%20Cue%20Object%20Reference))
  (if (and (not (Utilities|Array|ContainsItem (Variables|MusicComponents|GetplayOnNextBeat) soundCueToQueue)) (not (Variables|Default|GetmutexLocked)))
    (Utilities|Array|Add (Variables|MusicComponents|GetplayOnNextBeat) soundCueToQueue)))

(fn FadeOutandStopLoopCue
  (params (SoundCue :type Sound%20Cue%20Object%20Reference))
  (if (.ReturnValue (Utilities|Map|Find (Variables|MusicComponents|GetloopPlayers) SoundCue))
    (Utilities|Array|Add (Variables|MusicComponents|GetstopOnNextBeat) SoundCue))
  (return))

(fn PlayAllQueuedSounds
  (bind _playonnextbeat (Variables|MusicComponents|GetplayOnNextBeat))
  (bind _loopplayers (Variables|MusicComponents|GetloopPlayers))
  (for _array_element _playonnextbeat
    (if (.ReturnValue (Utilities|Map|Find _loopplayers _array_element))
      (if (not (Audio|Components|Audio|IsPlaying (.Value (Utilities|Map|Find _loopplayers _array_element))))
        (bind _returnvalue (Audio|SpawnSound2D _array_element :!label _label))
        (Utilities|Map|Add _loopplayers _array_element _returnvalue))
      (else
        (goto _label))))
  (Utilities|Array|Clear _playonnextbeat))

(fn StopAllSoundstobeQueued
  (bind _stoponnextbeat (Variables|MusicComponents|GetstopOnNextBeat))
  (for _array_element _stoponnextbeat
    (if (.ReturnValue (Utilities|Map|Find (Variables|MusicComponents|GetloopPlayers) _array_element))
      (Audio|Components|Audio|Stop (.Value (Utilities|Map|Find (Variables|MusicComponents|GetloopPlayers) _array_element)))
      (Components|DestroyComponent (.Value (Utilities|Map|Find (Variables|MusicComponents|GetloopPlayers) _array_element)))))
  (Utilities|Array|Clear _stoponnextbeat))